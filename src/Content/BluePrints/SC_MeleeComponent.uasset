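; Melee combo component for a Character, playing attack montages from X and Y input chains indexed by a shared counter.
; Begin/End functions gate the combo: presses in the input window queue the next attack, which fires during the transition window.
; Attack plays only when not falling.
; Pressing one button after the other immediately plays an AttackXY or AttackYX crossover montage, bypassing those checks and clearing the tracked montage.
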(event Custom|ChangeAttackYX
  (bind _attackcount (Variables|Default|GetAttackCount))
  (bind _attackyx (Variables|Default|GetAttackYX))
  (Variables|Default|SetbIsComboInputAccepting false)
  (Variables|Default|SetbIsTransitionCombo false)
  (Variables|Default|SetbIsNextAttack false)
  (if (Utilities|Array|IsValidIndex _attackyx _attackcount)
    (Animation|Montage|PlayMontage (Variables|/Script/Engine.Character|GetMesh (Variables|Default|GetOwnerCharacter)) (Utilities|Array|Get(acopy) _attackyx _attackcount)
      (:then
        (Variables|Default|SetCurrentAttackAnim 0)
        (Variables|Default|SetbIsChangeAttackY false)
        (Variables|Default|SetbIsChangeAttackX false)
        (Variables|Default|SetbIsAttackX false)))))

(event Custom|Attack
  (bind _attackanimsx (Variables|Default|GetAttackAnimsX))
  (bind _attackcount (Variables|Default|GetAttackCount))
  (bind _ownercharacter (Variables|Default|GetOwnerCharacter))
  (bind _attackanimy (Variables|Default|GetAttackAnimY))
  (bind _attackcount_2 (Variables|Default|GetAttackCount))
  (bind _output (Utilities|Array|Get(acopy) _attackanimsx _attackcount))
  (bind _output_2 (Utilities|Array|Get(acopy) _attackanimy _attackcount_2))
  (bind _mesh (Variables|/Script/Engine.Character|GetMesh _ownercharacter))
  (Variables|Default|SetbIsComboInputAccepting false)
  (Variables|Default|SetbIsTransitionCombo false)
  (Variables|Default|SetbIsNextAttack false)
  (if (not (AI|Components|NavMovement|IsFalling (Variables|/Script/Engine.Character|GetCharacterMovement (Variables|Default|GetOwnerCharacter))))
    (if (Variables|Default|GetbIsAttackX)
      (if (Utilities|Array|IsValidIndex _attackanimsx _attackcount)
        (Animation|Montage|PlayMontage _mesh _output
          (:then
            (Variables|Default|SetCurrentAttackAnim _output)
            (Variables|Default|SetbIsAttackX false))))
      (elif (Utilities|Array|IsValidIndex _attackanimy _attackcount_2)
        (Animation|Montage|PlayMontage _mesh _output_2
          (:then
            (Variables|Default|SetCurrentAttackAnim _output_2)
            (Variables|Default|SetbIsAttackX false)))))))

(event Custom|ChangeAttackXY
  (bind _attackxy (Variables|Default|GetAttackXY))
  (bind _attackcount (Variables|Default|GetAttackCount))
  (Variables|Default|SetbIsComboInputAccepting false)
  (Variables|Default|SetbIsTransitionCombo false)
  (Variables|Default|SetbIsNextAttack false)
  (if (Utilities|Array|IsValidIndex _attackxy _attackcount)
    (Animation|Montage|PlayMontage (Variables|/Script/Engine.Character|GetMesh (Variables|Default|GetOwnerCharacter)) (Utilities|Array|Get(acopy) _attackxy _attackcount)
      (:then
        (Variables|Default|SetCurrentAttackAnim 0)
        (Variables|Default|SetbIsChangeAttackX false)
        (Variables|Default|SetbIsChangeAttackY false)
        (Variables|Default|SetbIsAttackX false)))))

(event Input|EnhancedActionEvents|EnhancedInputActionIA_OnTriggerAtack_Combo_ActionX
  (params (ActionValue :type Boolean) (ElapsedSeconds :type Float%20%28double-precision%29) (TriggeredSeconds :type Float%20%28double-precision%29) (InputAction :type Input%20Action%20Object%20Reference :default "/Game/Input/Actions/IA_OnTriggerAtack_Combo_ActionX.IA_OnTriggerAtack_Combo_ActionX"))
  (Variables|Default|SetbIsAttackX true)
  (Variables|Default|SetbIsChangeAttackX true)
  (if (Variables|Default|GetbIsChangeAttackY)
    (CallFunction|ChangeAttackYX)
    (elif (CallFunction|IsAttacking)
      (if (Variables|Default|GetbIsComboInputAccepting)
        (if (not (Variables|Default|GetbIsNextAttack))
          (Variables|Default|SetbIsNextAttack true)
          (Math|Integer|IncrementInt (Variables|Default|GetAttackCount)
            (:%20%20
              (if (Variables|Default|GetbIsTransitionCombo)
                (CallFunction|Attack))))))
      (else
        (Variables|Default|SetAttackCount 0)
        (CallFunction|Attack)))))

(event Input|EnhancedActionEvents|EnhancedInputActionIA_OnTriggerAtack_Combo_ActionY
  (params (ActionValue :type Boolean) (ElapsedSeconds :type Float%20%28double-precision%29) (TriggeredSeconds :type Float%20%28double-precision%29) (InputAction :type Input%20Action%20Object%20Reference :default "/Game/Input/Actions/IA_OnTriggerAtack_Combo_ActionY.IA_OnTriggerAtack_Combo_ActionY"))
  (Variables|Default|SetbIsChangeAttackY true)
  (if (Variables|Default|GetbIsChangeAttackX)
    (CallFunction|ChangeAttackXY)
    (elif (CallFunction|IsAttacking)
      (if (Variables|Default|GetbIsComboInputAccepting)
        (if (not (Variables|Default|GetbIsNextAttack))
          (Variables|Default|SetbIsNextAttack true)
          (Math|Integer|IncrementInt (Variables|Default|GetAttackCount)
            (:%20%20
              (if (Variables|Default|GetbIsTransitionCombo)
                (CallFunction|Attack))))))
      (else
        (Variables|Default|SetAttackCount 0)
        (CallFunction|Attack)))))

(event EventBeginPlay
  (bind _asキャラクター (Utilities|Casting|CastToCharacter (Components|GetOwner)))
  (Variables|Default|SetOwnerCharacter _asキャラクター))

(fn IsAttacking
  (Variables|Default|GetCurrentAttackAnim
    (:then
      (return (== (Animation|Montage|GetCurrentActiveMontage (Components|SkeletalMesh|GetAnimInstance (Variables|/Script/Engine.Character|GetMesh (Variables|Default|GetOwnerCharacter)))) (Variables|Default|GetCurrentAttackAnim))))
    (:else
      (return false))))

(fn OnComboInputAcceptBegin
  (Variables|Default|SetbIsComboInputAccepting true))

(fn OnComboInputAcceptEnd
  (Variables|Default|SetbIsComboInputAccepting false))

(fn OnTransitionComboBegin
  (Variables|Default|SetbIsTransitionCombo true)
  (if (Variables|Default|GetbIsNextAttack)
    (CallFunction|Attack)))

(fn OnTransitionComboEnd
  (Variables|Default|SetbIsTransitionCombo false))